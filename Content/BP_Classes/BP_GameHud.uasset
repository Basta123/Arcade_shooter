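; HUD for the arcade shooter that draws life icons and the score, and shows a game-over widget when the game mode fires GameOver.
; DrawHUD reads health and points from the game mode each frame, placing elements with viewport-scale and anchor helpers.
; A hit-box click opens the pause menu and pauses the game, but the function drawing that button and hit box is disconnected.
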(event Custom|CustomEvent_0
  (bind _returnvalue (UserInterface|CreateWidget "/Game/UI/GameOverScreen/W_GameOver.W_GameOver_C" (Game|Player|GetOwningPlayerController)))
  (UserInterface|Viewport|AddtoViewport _returnvalue 0))

(event EventBeginPlay
  (bind _asbp_arcade_game_mode (Utilities|Casting|CastToBP_ArcadeGameMode (Game|GetGameMode)))
  (EventDispatchers|BindEventtoGameOver _asbp_arcade_game_mode (delegate Custom|CustomEvent_0)))

(event EventHitBoxClick
  (params (BoxName :type Name :default "None"))
  (Development|PrintString "Pause" true true "(R=0.671296,G=0.000000,B=0.055223,A=1.000000)" 5.0)
  (bind _returnvalue (UserInterface|CreateWidget "/Game/UI/PauseMenu/W_PauseMenu.W_PauseMenu_C" (Game|Player|GetOwningPlayerController)))
  (UserInterface|Viewport|AddtoViewport _returnvalue 0)
  (Game|SetGamePaused true))

(event EventDrawHUD
  (params (SizeX :type Integer) (SizeY :type Integer))
  (CallFunction|DrawHealths)
  (CallFunction|DrawPoints))

(event EventHitBoxBeginCursorOver
  (params (BoxName :type Name :default "None")))

(fn ConstructionScript)

(fn ScaledCoords
  (params (In :type Vector%202D%20Structure))
  (return (* In (Class|WidgetLayoutLibrary|GetViewportScale))))

(fn DrawHealths
  (bind _out (CallFunction|ScaledCoords "(X=64.000000,Y=64.000000)"))
  (for _index (range 0 (- (Class|GameHealthComponent|GetHealths (Variables|/Script/Arcade_shooter.Arcade_shooterGameModeBase|GetHealthsComponent (.AsArcade%20Shooter%20Game%20Mode%20Base (Utilities|Casting|CastToArcade_shooterGameModeBase (Game|GetGameMode))))) 1))
    (Canvas|DrawTexture "/Game/UI/live_icon.live_icon" (.x (CallFunction|ScaledCoords (Math|Vector2D|MakeVector2D (+ (* _index 74.0) 2e+01) 2e+01))) (.y (CallFunction|ScaledCoords (Math|Vector2D|MakeVector2D (+ (* _index 74.0) 2e+01) 2e+01))) (.x _out) (.y _out) 0.0 0.0 1.0 1.0 "(R=1.000000,G=1.000000,B=1.000000,A=1.000000)")))

(fn DrawPause
  (bind _out (CallFunction|ScaledCoords "(X=-84.000000,Y=20.000000)"))
  (bind _out_2 (CallFunction|ScaledCoords "(X=64.000000,Y=64.000000)"))
  (bind _out_3 (CallFunction|ApplyCoorsAnchor _out "(X=1.000000,Y=0.000000)"))
  (Canvas|DrawTexture "/Game/Assets/UI/Pause.Pause" (.x _out_3) (.y _out_3) (.x _out_2) (.y _out_2) 0.0 0.0 1.0 1.0 "(R=1.000000,G=1.000000,B=1.000000,A=1.000000)")
  (Class|HUD|AddHitBox (Math|Vector2D|MakeVector2D 64.0 64.0) (CallFunction|ScaledCoords "(X=64.000000,Y=64.000000)") "pp" false))

(fn ApplyCoorsAnchor
  (params (in :type Vector%202D%20Structure) (Anchor :type Vector%202D%20Structure))
  (return (+ in (* Anchor (Viewport|GetViewportSize)))))

(fn DrawPoints
  (bind _asbp_arcade_game_mode (Utilities|Casting|CastToBP_ArcadeGameMode (Game|GetGameMode)))
  (HUD|DrawText (Utilities|String|ToString(Integer) (Variables|/Script/Arcade_shooter.Arcade_shooterGameModeBase|GetGamePoint _asbp_arcade_game_mode)) "(R=1.000000,G=1.000000,B=1.000000,A=1.000000)" (.x (CallFunction|ApplyCoorsAnchor (CallFunction|ScaledCoords (Math|Vector2D|MakeVector2D (* (.OutWidth (Class|HUD|GetTextSize (Utilities|String|ToString(Integer) (Variables|/Script/Arcade_shooter.Arcade_shooterGameModeBase|GetGamePoint _asbp_arcade_game_mode)) 0 1.0)) -1.0) 2e+01)) "(X=0.500000,Y=0.000000)")) (.y (CallFunction|ApplyCoorsAnchor (CallFunction|ScaledCoords (Math|Vector2D|MakeVector2D (* (.OutWidth (Class|HUD|GetTextSize (Utilities|String|ToString(Integer) (Variables|/Script/Arcade_shooter.Arcade_shooterGameModeBase|GetGamePoint _asbp_arcade_game_mode)) 0 1.0)) -1.0) 2e+01)) "(X=0.500000,Y=0.000000)")) "/Game/Assets/UI/F_BigRoboto.F_BigRoboto" 1.0 false))