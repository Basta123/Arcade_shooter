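; Enemy pawn that homes in on the player pawn, which it caches on BeginPlay after calling the parent event.
; Each Tick it moves forward along local X by a fixed, unswept step that is not scaled by delta time.
; It yaws toward the player using the look-at delta clamped by RotMaxSpeed and scaled by delta time.
; The clamp is asymmetric, with the negative limit twice the positive one.
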(event EventTick
  (params (DeltaSeconds :type Float%20%28single-precision%29))
  (bind _rotmaxspeed (Variables|Default|GetRotMaxSpeed))
  (Utilities|IsValid (Variables|Default|GetPlayerPawn)
    (:Is%20Valid
      (Transformation|AddActorLocalOffset "5.000000,0.000000, 0" false false)
      (Transformation|AddActorLocalRotation (Math|Rotator|MakeRotator 0.0 0.0 (* (Math|Float|Clamp(Float) (.yaw (Math|Rotator|Delta(Rotator) (Math|Rotator|FindLookatRotation (Transformation|GetActorLocation) (Transformation|GetActorLocation (Variables|Default|GetPlayerPawn))) (Transformation|GetActorRotation))) (* -2.0 _rotmaxspeed) _rotmaxspeed) (Utilities|Time|GetWorldDeltaSeconds))) false false))))

(event EventBeginPlay
  (|CallParentFunction)
  (Variables|Default|SetPlayerPawn (Game|Player|GetPlayerPawn 0)))

(fn ConstructionScript)